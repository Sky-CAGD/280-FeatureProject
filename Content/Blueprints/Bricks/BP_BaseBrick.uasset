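; Base brick actor for a Breakout-style game, destroyed when a BP_Ball hits it.
; On a ball hit it adds its BrickScore through BP_GameInstance, notifies the level's BP_BrickManager that a brick was destroyed, then destroys itself.
; The construction script creates a dynamic material on the Cube and applies BrickColor to its Color parameter, so each brick can have its own color.
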(event Collision|EventHit
  (params (MyComp :type Primitive%20Component%20Object%20Reference) (Other :type Actor%20Object%20Reference) (OtherComp :type Primitive%20Component%20Object%20Reference) (bSelfMoved :type Boolean) (HitLocation :type Vector :default "0, 0, 0") (HitNormal :type Vector :default "0, 0, 0") (NormalImpulse :type Vector :default "0, 0, 0") (Hit :type Hit%20Result%20Structure%20%28by%20ref%29))
  ;[0 0 0 0.5] Destroy the brick when hit by a ball
  (Utilities|Casting|CastToBP_Ball Other)
  (Utilities|FlowControl|Sequence
    (:then_0
      ;[0.15 0.15 0.15 0.5] Increasing the score
      (bind _asbp_game_instance (Utilities|Casting|CastToBP_GameInstance (Game|GetGameInstance)))
      (Default|AddScore _asbp_game_instance (Variables|Default|GetBrickScore)))
    (:then_1
      ;[0.15 0.15 0.15 0.5] Decrease brick count and check if we won.
      (bind _returnvalue (Actor|GetActorOfClass "/Game/Blueprints/BP_BrickManager.BP_BrickManager_C"))
      (Default|BrickDestroyed _returnvalue))
    (:then_2
      ;[0.15 0.15 0.15 0.5] Destroy the brick that was hit. Potentially increase the ball speed.
      (Actor|DestroyActor))))

(fn ConstructionScript
  ;[0 0 0 0.5] Create dynamic 'BrickColor' parameter
  (bind _returnvalue (Rendering|Material|CreateDynamicMaterialInstance (Variables|Default|GetCube) 0 0 "None" :!class /Script/Engine.PrimitiveComponent))
  (Rendering|Material|SetVectorParameterValue _returnvalue "Color" (Variables|Default|GetBrickColor) :!class /Script/Engine.MaterialInstanceDynamic))